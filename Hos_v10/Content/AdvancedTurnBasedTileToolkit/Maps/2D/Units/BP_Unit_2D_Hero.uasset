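; Player hero unit for the 2D turn-based tile toolkit that uncovers fog, interacts with objects and equips gear.
; On selection it reveals unrevealed surroundings and picks the combat or free-roam ability based on initiative order size.
; Simulated tile entry triggers grid object interactions and reveals tiles through the 2D grid manager.
; Equip applies item stats, sounds and projectile, then spawns an equip action to update the puppet's sprite.
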(event `self.ReceiveBeginPlay`
  (`parent.ReceiveBeginPlay`)
  (bind _asbp_grid_manager_2d (cast `/Game/AdvancedTurnBasedTileToolkit/Maps/2D/Core/BP_GridManager_2D` (`self.GridManagerRef`)))
  (set `self.GridManager2DRef` _asbp_grid_manager_2d))

(event `/Game/AdvancedTurnBasedTileToolkit/Core/BPI_Initiative.SelectActor`
  (if (not (`BlueprintSetLibrary.Set_Contains` (`/Game/AdvancedTurnBasedTileToolkit/Maps/2D/Core/BP_GridManager_2D.RevealedGridIndexes` (`self.GridManager2DRef`)) (`self.GridIndex`)))
    (`KismetSystemLibrary.Delay` 0.0)
    (`/Game/AdvancedTurnBasedTileToolkit/Maps/2D/Core/BP_GridManager_2D.RevealTiles` (`self.GridManager2DRef`) (`self.GridIndex`)))
  (set `self.DefaultAbility` (select `bool` (> (`KismetArrayLibrary.Array_Length` (`/Game/AdvancedTurnBasedTileToolkit/Core/BP_TurnManager.InitiativeOrderActors` (`.TurnManager` (`/Game/AdvancedTurnBasedTileToolkit/Core/BPFL_Singletons.GetTurnManager`)))) 1) :`false` "/Game/AdvancedTurnBasedTileToolkit/Core/Abilities/BP_AbilityBase_FreeRoam.BP_AbilityBase_FreeRoam_C" :`true` "/Game/AdvancedTurnBasedTileToolkit/Maps/2D/Abilities/BP_Ability_2D.BP_Ability_2D_C" :!type "/Game/AdvancedTurnBasedTileToolkit/Core/Abilities/BP_AbilityBase Class Reference"))
  (`parent.SelectActor`))

(fn `Equip`
  (params (EquipmentActor :type "Actor Object Reference") (EquipmentData :type "/Game/AdvancedTurnBasedTileToolkit/Maps/2D/Items/FEquipment2D Structure"))
  (bind (_groundsprite _equipsprite _damage _armor _equipmentslot _range) (break `/Game/AdvancedTurnBasedTileToolkit/Maps/2D/Items/FEquipment2D` EquipmentData))
  (bind (_groundsprite_2 _equipsprite_2 _damage_2 _armor_2 _equipmentslot_2 _range_2 _attacksound _hitsound _projectile) (break `/Game/AdvancedTurnBasedTileToolkit/Maps/2D/Items/FEquipment2D` (`local.EquipmentData`)))
  (bind (_groundsprite_3 _equipsprite_3 _damage_3 _armor_3 _equipmentslot_3) (break `/Game/AdvancedTurnBasedTileToolkit/Maps/2D/Items/FEquipment2D` (`local.EquipmentData`)))
  (if (> _damage 0.0)
    (set `self.Damage` _damage))
  (set `self.Armor` (+ (`self.Armor`) _armor))
  (set `self.Range` _range)
  (`/Engine/EditorBlueprintResources/StandardMacros.IsValid` _attacksound
    (:`Is Valid`
      (set `self.AttackSound` _attacksound))
    (:`Is Not Valid`
      _))
  (`/Engine/EditorBlueprintResources/StandardMacros.IsValid` _hitsound
    (:`Is Valid`
      (set `self.HitSound` _hitsound))
    (:`Is Not Valid`
      _))
  (`/Engine/EditorBlueprintResources/StandardMacros.IsValid` _projectile
    (:`Is Valid`
      (set `self.Projectile` _projectile))
    (:`Is Not Valid`
      _))
  (bind _asbp_2d_puppet_hero (cast `/Game/AdvancedTurnBasedTileToolkit/Maps/2D/Units/BP_2D_Puppet_Hero` (`self.Puppet`))
    (:`then`
      (`|SpawnActorFromClass` "/Game/AdvancedTurnBasedTileToolkit/Maps/2D/Actions/BP_Action_Equip_2D.BP_Action_Equip_2D_C" (`KismetMathLibrary.MakeTransform` (0.0 0.0 0.0)) "Undefined" "OverrideRootScale" null _asbp_2d_puppet_hero _equipmentslot_3 _equipsprite_3 (`local.EquipmentActor`) -1.0 "NewEnumerator0" null)
      (return))
    (:`CastFailed`
      (return))))

(fn `SimulateEnterTile`
  (params (EnteringGridIndex :type Integer) (ExitingGridIndex :type Integer) (PathIndexes :type "Array of Integer (by ref)"))
  (`parent.SimulateEnterTile` EnteringGridIndex ExitingGridIndex PathIndexes)
  (`/Game/AdvancedTurnBasedTileToolkit/Core/Grid/BP_GridManager.InteractWithObjects` (`self.GridManagerRef`) (`local.EnteringGridIndex`) self null true "NewEnumerator1" -1)
  (`/Game/AdvancedTurnBasedTileToolkit/Maps/2D/Core/BP_GridManager_2D.RevealTiles` (`self.GridManager2DRef`) (`local.EnteringGridIndex`))
  (return))

(fn `UserConstructionScript`
  (`parent.UserConstructionScript`))