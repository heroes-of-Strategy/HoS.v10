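; BP_Action_ShowSelection is a turn-based toolkit action that presents the selected actor to the player.
; When played, it sets that actor as the turn manager's ActiveActorAnimate and tells the player pawn to follow it.
; It then marks the actor through the player controller's grid UI, fetched with a class override, and ends the action immediately.
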(event `self.PlayAction`
  (set `/Game/AdvancedTurnBasedTileToolkit/Core/BP_TurnManager.ActiveActorAnimate` (`self.SelectedActor`) (`.TurnManager` (`/Game/AdvancedTurnBasedTileToolkit/Core/BPFL_Singletons.GetTurnManager`)))
  (message `/Game/AdvancedTurnBasedTileToolkit/Core/BPI_CameraControls.FollowActor` (`GameplayStatics.GetPlayerPawn` 0) (`self.SelectedActor`))
  (bind _gridui (message `/Game/AdvancedTurnBasedTileToolkit/Core/BPI_Ability.GetGridUi` (`GameplayStatics.GetPlayerController` 0) (`self.GridUIClassOverride`)))
  (`/Game/AdvancedTurnBasedTileToolkit/Core/GridUI/BP_GridUI.MarkActor` _gridui (`self.SelectedActor`))
  (`self.EndAction` true))

(fn `UserConstructionScript`
  (`parent.UserConstructionScript`))