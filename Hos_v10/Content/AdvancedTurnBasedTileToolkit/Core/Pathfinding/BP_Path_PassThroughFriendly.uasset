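; Pathfinding variant for the turn-based tile toolkit that, as its name indicates, lets movement pass through friendly units.
; AddTileIfValid records tiles within the move budget in Paths with cost and parent, then queues them in the child open list.
; Occupied tiles are also logged in ReachableUnitIndexes but still expand the search.
; This function itself checks no faction, only cost and occupancy.
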(fn `AddTileIfValid`
  (params (EdgeIndex :type "Integer (by ref)") (TotalCost :type "Integer (by ref)") (ParentIndex :type "Integer (by ref)") (Move :type "Integer (by ref)") (Paths :type "Map of Integer to /Game/AdvancedTurnBasedTileToolkit/Core/Grid/FPathfinding Structure (by ref)") (OpenListChildTiles :type "Array of /Game/AdvancedTurnBasedTileToolkit/Core/Grid/FPathfindingIndex Structure (by ref)"))
  (if (<= TotalCost Move)
    (`BlueprintMapLibrary.Map_Add` (`local.Paths`) (`local.EdgeIndex`) (make `/Game/AdvancedTurnBasedTileToolkit/Core/Grid/FPathfinding` (`local.TotalCost`) (`local.ParentIndex`)))
    (if (`BlueprintMapLibrary.Map_Contains` (`/Game/AdvancedTurnBasedTileToolkit/Core/Grid/BP_GridManager.GridUnits` (`self.GridManagerRef`)) (`local.EdgeIndex`))
      (`BlueprintSetLibrary.Set_Add` (`self.ReachableUnitIndexes`) (`local.EdgeIndex`)))
    (`KismetArrayLibrary.Array_Add` (`local.OpenListChildTiles`) (make `/Game/AdvancedTurnBasedTileToolkit/Core/Grid/FPathfindingIndex` (`local.EdgeIndex`) (`local.TotalCost`) (`local.ParentIndex`)))
    (else
      (return))))