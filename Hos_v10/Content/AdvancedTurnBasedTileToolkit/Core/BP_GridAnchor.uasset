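; BP_GridAnchor is a scene component that anchors its owning actor to the tile grid of BP_GridManager.
; ExternalConstuctionScript traces for the tile closest to the owner, moves the component there unless IgnoreSnapToCustomGrid is set, and derives GridIndex from that tile location.
; PlaceActorAtAnchor is effectively empty, as its logic for moving the owner to the offset snapped position is disconnected.
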(event `ExternalConstuctionScript`
  (bind _returnvalue (`self.GetOwner`))
  (bind _returnvalue_2 (`GameplayStatics.GetActorOfClass` "/Game/AdvancedTurnBasedTileToolkit/Core/Grid/BP_GridManager.BP_GridManager_C"))
  (`/Engine/EditorBlueprintResources/StandardMacros.IsValid` _returnvalue_2
    (:`Is Valid`
      (if (not (`self.bIgnoreSnapToCustomGrid`))
        (bind _snaplocation (`/Game/AdvancedTurnBasedTileToolkit/Core/Grid/BP_GridManager.FindClosestTileToSnapToTrace` _returnvalue_2 (`Actor.K2_GetActorLocation` _returnvalue) (`|MakeArray` _returnvalue)))
        (`self.K2_SetWorldLocation` self _snaplocation false false))
      (set `self.GridIndex` (`/Game/AdvancedTurnBasedTileToolkit/Core/Grid/BP_GridManager.ConvertLocationToIndex3D` _returnvalue_2 _snaplocation)))))

(fn `PlaceActorAtAnchor`)