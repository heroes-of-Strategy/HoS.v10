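; BP_Actor_Puppet_Debug is a puppet actor that gives a visual stand-in for its parent BP_Unit.
; Its construction script casts the parent actor to BP_Unit and configures the look from that unit's stats.
; Range above one selects the standard animation Blueprint and shows the weapon; otherwise it uses the melee one and hides it.
; Faction picks the body and chest-logo materials, and the event graph is unused.
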(fn `UserConstructionScript`
  (`parent.UserConstructionScript`)
  (bind _asbp_unit (cast `/Game/AdvancedTurnBasedTileToolkit/Core/Units/BP_Unit` (`self.GetParentActor`)))
  (bind _range (`/Game/AdvancedTurnBasedTileToolkit/Core/Units/BP_Unit.Range` _asbp_unit))
  (`SkeletalMeshComponent.SetAnimInstanceClass` (`self.UnitMesh`) (select `bool` (> _range 1) :`false` "/Game/AdvancedTurnBasedTileToolkit/Units/ABP_Unit_Melee.ABP_Unit_Melee_C" :`true` "/Game/AdvancedTurnBasedTileToolkit/Units/ABP_Unit.ABP_Unit_C" :!type "Object Class Reference"))
  (`SceneComponent.SetVisibility` (`self.Weapon`) (> _range 1) false)
  (bind _faction (`/Game/AdvancedTurnBasedTileToolkit/Core/Units/BP_Unit.Faction` _asbp_unit))
  (`PrimitiveComponent.SetMaterial` (`self.UnitMesh`) 0 (select `/Game/AdvancedTurnBasedTileToolkit/Core/Units/EFaction` _faction :`NewEnumerator3` "/Game/AdvancedTurnBasedTileToolkit/Core/Tiles/M_Grey_Transparent.M_Grey_Transparent" :`NewEnumerator0` "/Game/AdvancedTurnBasedTileToolkit/Units/MI_UE4Man_Body_Green.MI_UE4Man_Body_Green" :`NewEnumerator1` "/Game/AdvancedTurnBasedTileToolkit/Units/MI_UE4Man_Body_Red.MI_UE4Man_Body_Red" :!type "MaterialInterface Object Reference"))
  (`PrimitiveComponent.SetMaterial` (`self.UnitMesh`) 1 (select `/Game/AdvancedTurnBasedTileToolkit/Core/Units/EFaction` _faction :`NewEnumerator3` "/Game/AdvancedTurnBasedTileToolkit/Core/Tiles/M_Grey_Transparent.M_Grey_Transparent" :`NewEnumerator0` "/Game/AdvancedTurnBasedTileToolkit/Units/MI_UE4Man_ChestLogo_Green.MI_UE4Man_ChestLogo_Green" :`NewEnumerator1` "/Game/AdvancedTurnBasedTileToolkit/Units/MI_UE4Man_ChestLogo_Red.MI_UE4Man_ChestLogo_Red" :`NewEnumerator4` "/Game/AdvancedTurnBasedTileToolkit/Units/MI_UE4Man_ChestLogo.MI_UE4Man_ChestLogo" :!type "MaterialInterface Object Reference")))