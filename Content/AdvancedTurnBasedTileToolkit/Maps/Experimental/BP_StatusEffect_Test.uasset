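; BP_StatusEffect_Test is an experimental test status effect for the Advanced Turn Based Tile Toolkit that logs when its turn-start and turn-end hooks fire.
; It handles the RunonTurnStart and RunonTurnEnd events by printing "Start:" or "End:" followed by the owning unit's display name.
; It applies no gameplay effect, and its construction script only calls the parent's.
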(event `self.RunOnTurnStart`
  (`KismetSystemLibrary.PrintString` (`KismetStringLibrary.Concat_StrStr` "Start: " (`KismetSystemLibrary.GetDisplayName` (`self.OwningUnit`)))))

(event `self.RunOnTurnEnd`
  (`KismetSystemLibrary.PrintString` (`KismetStringLibrary.Concat_StrStr` "End: " (`KismetSystemLibrary.GetDisplayName` (`self.OwningUnit`)))))

(fn `UserConstructionScript`
  (`parent.UserConstructionScript`))