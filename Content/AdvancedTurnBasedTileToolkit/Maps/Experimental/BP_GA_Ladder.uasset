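; Ladder grid actor for the turn-based tile toolkit that links its own tile to the one at its top.
; The construction script picks edge costs from yaw, traces down from TopLocation to find the upper tile, and adds two-way custom edges.
; It also snaps the Top component to the hit height and stacks instanced sections below it.
; BeginPlay repeats the trace to register direction-specific special edges with the grid manager.
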(event `self.ReceiveBeginPlay`
  (bind _gridmanagerref (`self.GridManagerRef`))
  (bind _returnvalue (`KismetMathLibrary.TransformLocation` (`self.GetTransform`) (`self.TopLocation`)))
  (bind (_outhit _returnvalue_2) (`KismetSystemLibrary.LineTraceSingle` _returnvalue (- _returnvalue (* (`self.GetActorUpVector` _gridmanagerref) (+ (`KismetMathLibrary.Abs` (`/Game/AdvancedTurnBasedTileToolkit/Core/Grid/BP_GridManager.MaxGridHeight` _gridmanagerref)) (`KismetMathLibrary.Abs` (`/Game/AdvancedTurnBasedTileToolkit/Core/Grid/BP_GridManager.MinGridHeight` _gridmanagerref))))) "TraceTypeQuery1"))
  (if _returnvalue_2
    (bind _index (`/Game/AdvancedTurnBasedTileToolkit/Core/Grid/BP_GridManager.ConvertLocationToIndex3D` (`self.GridManagerRef`) (`.Location` (`GameplayStatics.BreakHitResult` _outhit))))
    (`/Game/AdvancedTurnBasedTileToolkit/Core/BPML_ATBTT.MakeLocalVariable` _index)
    (`/Game/AdvancedTurnBasedTileToolkit/Core/Grid/BP_GridManager.AddSpecialEdge` (`self.GridManagerRef`) (`self.GridIndex`) _index "NewEnumerator2")
    (`/Game/AdvancedTurnBasedTileToolkit/Core/Grid/BP_GridManager.AddSpecialEdge` (`self.GridManagerRef`) _index (`self.GridIndex`) "NewEnumerator3")))

(fn `AddInstanceStep`
  (params (StepIndex :type Integer) (Ism :type "InstancedStaticMeshComponent Object Reference"))
  (bind (_returnvalue_location _returnvalue_rotation _returnvalue_scale) (`KismetMathLibrary.BreakTransform` (`SceneComponent.K2_GetComponentToWorld` Ism)))
  (`InstancedStaticMeshComponent.AddInstanceWorldSpace` Ism (`KismetMathLibrary.MakeTransform` (- (`SceneComponent.K2_GetComponentLocation` (`self.Top`)) (`KismetMathLibrary.MakeVector` 0.0 0.0 (* StepIndex (`self.StepHeight`)))) _returnvalue_rotation _returnvalue_scale)))

(fn `UserConstructionScript`
  (bind (_returnvalue_roll _returnvalue_pitch _returnvalue_yaw) (`KismetMathLibrary.BreakRotator` (`self.K2_GetActorRotation`)))
  (bind _top (`self.Top`))
  (bind _gridmanagerref (`self.GridManagerRef`))
  (bind (_returnvalue_x _returnvalue_y _returnvalue_z) (`KismetMathLibrary.BreakVector` (`SceneComponent.K2_GetComponentLocation` (`self.GridAnchor`))))
  (bind _returnvalue (`KismetMathLibrary.TransformLocation` (`self.GetTransform`) (`self.TopLocation`)))
  (bind (_returnvalue_x_2 _returnvalue_y_2) (`KismetMathLibrary.BreakVector` (`SceneComponent.K2_GetComponentLocation` _top)))
  (set `self.EdgeCost` (select `int` (`KismetMathLibrary.FFloor` (/ (mod (+ _returnvalue_yaw 405.0) 360.0) 90.0)) :`0` (make `/Game/AdvancedTurnBasedTileToolkit/Core/Tiles/FTileEdges` 1 1 0 1 1 0 0 1) :`1` (make `/Game/AdvancedTurnBasedTileToolkit/Core/Tiles/FTileEdges` 1 1 1 0 1 1) :`2` (make `/Game/AdvancedTurnBasedTileToolkit/Core/Tiles/FTileEdges` 0 1 1 1 0 1 1) :`3` (make `/Game/AdvancedTurnBasedTileToolkit/Core/Tiles/FTileEdges` 1 0 1 1 0 0 1 1) :!type "/Game/AdvancedTurnBasedTileToolkit/Core/Tiles/FTileEdges Structure"))
  (`parent.UserConstructionScript`)
  (`|ExecutionSequence`
    (:`then_1`
      (`KismetArrayLibrary.Array_Clear` (`self.CustomEdges`))
      (bind (_outhit _returnvalue_2) (`KismetSystemLibrary.LineTraceSingle` _returnvalue (- _returnvalue (* (`self.GetActorUpVector` _gridmanagerref) (+ (`KismetMathLibrary.Abs` (`/Game/AdvancedTurnBasedTileToolkit/Core/Grid/BP_GridManager.MaxGridHeight` _gridmanagerref)) (`KismetMathLibrary.Abs` (`/Game/AdvancedTurnBasedTileToolkit/Core/Grid/BP_GridManager.MinGridHeight` _gridmanagerref))))) "TraceTypeQuery1"))
      (if _returnvalue_2
        (bind ___ (`/Game/AdvancedTurnBasedTileToolkit/Core/BPML_ATBTT.MakeLocalVariable` (`/Game/AdvancedTurnBasedTileToolkit/Core/Grid/BP_GridManager.ConvertLocationToIndex3D` (`self.GridManagerRef`) (`.Location` (`GameplayStatics.BreakHitResult` _outhit)))))
        (`KismetArrayLibrary.Array_Add` (`self.CustomEdges`) (make `/Game/AdvancedTurnBasedTileToolkit/Core/Grid/FCustomEdge` (`self.GridIndex`) ___ 1))
        (`KismetArrayLibrary.Array_Add` (`self.CustomEdges`) (make `/Game/AdvancedTurnBasedTileToolkit/Core/Grid/FCustomEdge` ___ (`self.GridIndex`) 1))
        (bind _z (.z (`.Location` (`GameplayStatics.BreakHitResult` _outhit))))
        (`SceneComponent.K2_SetWorldLocation` _top (`KismetMathLibrary.MakeVector` _returnvalue_x_2 _returnvalue_y_2 _z) false false)
        (for _index (range 1 (+ (+ (`KismetMathLibrary.FTrunc` (/ (- _z _returnvalue_z) (`self.StepHeight`))) 1) 1))
          (`self.AddInstanceStep` _index (`self.Section`)))))))