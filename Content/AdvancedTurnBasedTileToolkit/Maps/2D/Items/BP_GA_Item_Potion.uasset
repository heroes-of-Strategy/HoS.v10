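; Healing potion grid actor for the 2D tile toolkit, consumed once when a player-controlled unit interacts with it; AI units are ignored.
; Interact immediately raises the unit's health, capped at its maximum, then queues a Drink action and the potion's destruction.
; AnimateAction plays the visual result separately from the game logic, updating the health bar, hiding the potion and playing a sound.
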(event `/Game/AdvancedTurnBasedTileToolkit/Core/Grid/BPI_Interact.Interact`
  (params (TriggeringActor :type "Actor Object Reference") (InteractionType :type "/Game/AdvancedTurnBasedTileToolkit/Core/Grid/EInteract Enum" :default "NewEnumerator0") (CurrentPathIndex :type Integer))
  (bind _asbp_unit (cast `/Game/AdvancedTurnBasedTileToolkit/Core/Units/BP_Unit` TriggeringActor))
  (if (not (`/Game/AdvancedTurnBasedTileToolkit/Core/Units/BP_Unit.bAIControlled` _asbp_unit))
    (`/Engine/EditorBlueprintResources/StandardMacros.DoOnce` false
      (:`Completed`
        (set `/Game/AdvancedTurnBasedTileToolkit/Core/Units/BP_Unit.CurrentHealth` (`KismetMathLibrary.FMin` (`/Game/AdvancedTurnBasedTileToolkit/Core/Units/BP_Unit.MaxHealth` _asbp_unit) (+ (`/Game/AdvancedTurnBasedTileToolkit/Core/Units/BP_Unit.CurrentHealth` _asbp_unit) (`self.HealAmount`))) _asbp_unit)
        (`/Game/AdvancedTurnBasedTileToolkit/Core/BPML_ATBTT.QueueAction` :`Executing Object` self :`Action Name` "Drink" :`Instant Deactivate` true :`Floats` (`|MakeArray` (`self.HealAmount`)) :`Units` (`|MakeArray` _asbp_unit))
        (`/Game/AdvancedTurnBasedTileToolkit/Core/BPML_ATBTT.QueueDestroy` (`|MakeArray` self :!type "Object Object Reference"))))))

(event `/Game/AdvancedTurnBasedTileToolkit/Core/BPI_Action.AnimateAction`
  (params (Action :type "/Game/AdvancedTurnBasedTileToolkit/Core/FAction Structure"))
  (bind (_executingobject _actionname _binstantdeactivate _atcustomindex _bwithprevious _activationdelay _booleans _integers _floats _strings _vectors _transforms _actors _units) (break `/Game/AdvancedTurnBasedTileToolkit/Core/FAction` Action))
  (bind _asbp_unit_2d (cast `/Game/AdvancedTurnBasedTileToolkit/Maps/2D/Units/BP_Unit_2D` (`|GetArrayItem` _units)))
  (`/Game/AdvancedTurnBasedTileToolkit/Maps/2D/Units/BP_Unit_2D.ModifyHealthBar` _asbp_unit_2d (`|GetArrayItem` _floats))
  (`self.SetActorHiddenInGame` true)
  (`GameplayStatics.PlaySound2D` "/Game/AdvancedTurnBasedTileToolkit/Maps/2D/Items/A_Potion.A_Potion" 1.0 1.0 0.0 null null))

(fn `UserConstructionScript`
  (`parent.UserConstructionScript`))