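; Equippable item for the 2D tile-based game that gives its gear to a hero unit interacting with it.
; On the first such interaction it calls Equip on the hero with its stats, sprite, type, sounds and projectile.
; It then queues its own Destroy action and a DestroyActors action on the action manager.
; AnimateAction handles the visual side, hiding the item and playing a potion sound.
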(event `/Game/AdvancedTurnBasedTileToolkit/Core/Grid/BPI_Interact.Interact`
  (params (TriggeringActor :type "Actor Object Reference") (InteractionType :type "/Game/AdvancedTurnBasedTileToolkit/Core/Grid/EInteract Enum" :default "NewEnumerator0") (CurrentPathIndex :type Integer))
  (bind _asbp_unit_2d_hero (cast `/Game/AdvancedTurnBasedTileToolkit/Maps/2D/Units/BP_Unit_2D_Hero` TriggeringActor))
  (`/Engine/EditorBlueprintResources/StandardMacros.DoOnce` false
    (:`Completed`
      (`/Game/AdvancedTurnBasedTileToolkit/Maps/2D/Units/BP_Unit_2D_Hero.Equip` _asbp_unit_2d_hero (`self.Damage`) (`self.Armor`) (`self.EquipSprite`) (`self.EquipType`) (`self.Range`) (`self.AttackSound`) (`self.HitSound`) (`self.Projectile`))
      (`/Game/AdvancedTurnBasedTileToolkit/Core/BPML_ATBTT.QueueAction` self "Destroy" "NewEnumerator0" true)
      (bind _actionmanager (`/Game/AdvancedTurnBasedTileToolkit/Core/BPML_Singletons.GetActionManager`))
      (`/Game/AdvancedTurnBasedTileToolkit/Core/BPML_ATBTT.QueueAction` :`Executing Object` _actionmanager :`Action Name` "DestroyActors" :`Instant Deactivate` true :`Actors` (`|MakeArray` self :!type "Actor Object Reference")))))

(event `/Game/AdvancedTurnBasedTileToolkit/Core/BPI_Action.AnimateAction`
  (params (Action :type "/Game/AdvancedTurnBasedTileToolkit/Core/FAction Structure"))
  (switch `name` (`.ActionName_37_58E425AA41088A6D07425C9F0FBA2C3F` (break `/Game/AdvancedTurnBasedTileToolkit/Core/FAction` Action))
    (:`Destroy`
      (`self.SetActorHiddenInGame` true)
      (`GameplayStatics.PlaySound2D` "/Game/AdvancedTurnBasedTileToolkit/Maps/2D/Items/A_Potion.A_Potion" 1.0 1.0 0.0 null null))))

(fn `UserConstructionScript`
  (`parent.UserConstructionScript`))