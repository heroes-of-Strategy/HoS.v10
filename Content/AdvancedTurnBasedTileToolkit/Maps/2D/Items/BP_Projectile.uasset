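; BP_Projectile is a 2D projectile actor in the Advanced Turn Based Tile Toolkit that flies to a Target location.
; On BeginPlay it faces the target, applies its sprite and unhides, then moves its root via MoveComponentTo over a duration of distance divided by MovementSpeed, giving constant speed.
; On arrival it plays a 2D hit sound, hides itself and calls EndAction.
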(event `self.ReceiveBeginPlay`
  (bind _returnvalue (`self.K2_GetActorLocation`))
  (bind _target (`self.Target`))
  (`self.K2_SetActorRotation` (`KismetMathLibrary.FindLookAtRotation` (`self.K2_GetActorLocation`) (`self.Target`)))
  (`PaperSpriteComponent.SetSprite` (`self.ProjectileSprite`) (`self.Sprite`))
  (`self.SetActorHiddenInGame` false)
  (`KismetSystemLibrary.MoveComponentTo` (`self.DefaultSceneRoot`) _target (`KismetMathLibrary.FindLookAtRotation` _returnvalue _target) false false (/ (`KismetMathLibrary.VSize` (- _target _returnvalue)) (`self.MovementSpeed`)))
  (`GameplayStatics.PlaySound2D` (`self.HitSound`) 1.0 1.0 0.0 null null)
  (`self.SetActorHiddenInGame` true)
  (`/Game/AdvancedTurnBasedTileToolkit/Core/BPML_ATBTT.EndAction`))

(fn `UserConstructionScript`)