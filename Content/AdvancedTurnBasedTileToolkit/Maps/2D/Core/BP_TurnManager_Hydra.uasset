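; Turn manager subclass from the 2D maps of the Advanced Turn Based Tile Toolkit that customizes turn animation and game-over text for Hydra units.
; Animated "Store Turn Info" actions record the turn and active actor, and both these and "Show Selection" make the player pawn follow the action's actor.
; Other actions defer to the parent.
; Game over displays VICTORY through the HUD if the remaining unit is exactly the Hydra class, otherwise GAME OVER.
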(event `/Game/AdvancedTurnBasedTileToolkit/Core/BPI_Action.AnimateAction`
  (params (Action :type "/Game/AdvancedTurnBasedTileToolkit/Core/FAction Structure"))
  (bind (_executingobject _actionname _binstantdeactivate _atcustomindex _bwithprevious _activationdelay _booleans _integers _floats _strings _vectors _transforms _actors) (break `/Game/AdvancedTurnBasedTileToolkit/Core/FAction` Action))
  (bind _output (`|GetArrayItem` _actors))
  (switch `name` _actionname
    (:`Default`
      (`parent.AnimateAction` Action))
    (:`StoreTurnInfo`
      (set `self.CurrentTurnAnimate` (`|GetArrayItem` _integers))
      (set `self.ActiveActorAnimate` _output)
      (message `/Game/AdvancedTurnBasedTileToolkit/Core/BPI_CameraControls.FollowActor` (`GameplayStatics.GetPlayerPawn` 0) _output :!label _label))
    (:`ShowSelection`
      (goto _label))))

(event `self.DisplayGameOver`
  (params (RemainingUnit :type "/Game/AdvancedTurnBasedTileToolkit/Core/Units/BP_Unit Object Reference"))
  (bind _asbp_hud_atbtt (cast `/Game/AdvancedTurnBasedTileToolkit/Core/UI/BP_HUD_ATBTT` (`PlayerController.GetHUD` (`GameplayStatics.GetPlayerController` 0))))
  (if (== (`GameplayStatics.GetObjectClass` RemainingUnit) "/Game/AdvancedTurnBasedTileToolkit/Maps/2D/Units/BP_Unit_2D_Hydra.BP_Unit_2D_Hydra_C")
    (bind _wbpatbttref (`/Game/AdvancedTurnBasedTileToolkit/Core/UI/BP_HUD_ATBTT.WbpAtbttRef` _asbp_hud_atbtt))
    (`/Game/AdvancedTurnBasedTileToolkit/Core/UI/WBP_ATBTT.DisplayCenterText` _wbpatbttref "VICTORY!" false 0.0)
    (else
      (`/Game/AdvancedTurnBasedTileToolkit/Core/UI/WBP_ATBTT.DisplayCenterText` _wbpatbttref "GAME OVER" false 0.0))))

(fn `UserConstructionScript`
  (`parent.UserConstructionScript`))