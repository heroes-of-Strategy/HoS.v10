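; 2D hero unit for the turn-based tile toolkit, extending a parent unit with equipment, armor and tile revealing.
; Movement simulates the path first, revealing tiles, triggering object interactions and queuing a step animation per tile, later played by a timeline.
; Equip updates combat stats immediately and queues the layered sprite swap.
; Armor reduces incoming damage, and animation overrides handle health bar, death and hiding gear sprites.
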(event `/Game/AdvancedTurnBasedTileToolkit/Core/BPI_Initiative.SelectActor`
  (`|ExecutionSequence`
    (:`then_0`
      (`/Engine/EditorBlueprintResources/StandardMacros.DoOnce` false
        (:`Completed`
          (`/Game/AdvancedTurnBasedTileToolkit/Maps/2D/Core/BP_GridManager_2D.RevealTiles` (`self.GridManager2DRef`) (`self.GridIndex`)))))
    (:`then_1`
      (`parent.SelectActor`))))

(event `/Game/AdvancedTurnBasedTileToolkit/Core/BPI_Action.AnimateAction`
  (params (Action :type "/Game/AdvancedTurnBasedTileToolkit/Core/FAction Structure"))
  (bind (_executingobject _actionname _binstantdeactivate _atcustomindex _bwithprevious _activationdelay _booleans _integers _floats _strings _vectors _transforms _actors _units _objects) (break `/Game/AdvancedTurnBasedTileToolkit/Core/FAction` Action))
  (bind (_returnvalue_x _returnvalue_y _returnvalue_z) (`KismetMathLibrary.BreakVector` (`self.K2_GetActorLocation`)))
  (bind _output (`|GetArrayItem` _integers))
  (switch `name` _actionname
    (:`Default`
      (`parent.AnimateAction` Action :!label _label))
    (:`MoveStep`
      (`/Game/AdvancedTurnBasedTileToolkit/Core/Grid/BP_GridManager.OnUnitExitTileAnimate` (`self.GridManagerRef`) self (- _output 1))
      (bind ___ (`/Game/AdvancedTurnBasedTileToolkit/Core/BPML_ATBTT.MakeLocalVariable` (`self.K2_GetActorLocation`)))
      (bind (_direction _movetrack) (`Timeline|TL_MoveStep` :!via `PlayFromStart`)
        (:`Update`
          (bind (_returnvalue_x_2 _returnvalue_y_2) (`KismetMathLibrary.BreakVector` (`KismetMathLibrary.VLerp` ___ (`|GetArrayItem` _vectors) _movetrack)))
          (`self.K2_SetActorLocation` (`KismetMathLibrary.MakeVector` _returnvalue_x_2 _returnvalue_y_2 _returnvalue_z)))
        (:`Finished`
          (`/Game/AdvancedTurnBasedTileToolkit/Core/Grid/BP_GridManager.OnUnitEnterTileAnimate` (`self.GridManagerRef`) self _output)
          (`GameplayStatics.PlaySound2D` "/Game/AdvancedTurnBasedTileToolkit/Maps/2D/Units/A_Step.A_Step" 1.0 1.0 0.0 null null)
          (`/Game/AdvancedTurnBasedTileToolkit/Core/BPML_ATBTT.EndAction`))))
    (:`Equip`
      (bind _aspaper_sprite (cast `PaperSprite` (`|GetArrayItem` _objects)))
      (`PaperSpriteComponent.SetSprite` (select `int` (`|GetArrayItem` _integers) :`0` (`self.WeaponSprite`) :`1` (`self.ArmorSprite`) :`2` (`self.ShieldSprite`) :`3` (`self.HelmSprite`) :`4` (`self.BootsSprite`)) _aspaper_sprite))
    (:`Death`
      (`|ExecutionSequence`
        (:`then_0`
          (`SceneComponent.SetHiddenInGame` (`self.WeaponSprite`) true false)
          (`SceneComponent.SetHiddenInGame` (`self.HelmSprite`) true false)
          (`SceneComponent.SetHiddenInGame` (`self.ArmorSprite`) true false)
          (`SceneComponent.SetHiddenInGame` (`self.ShieldSprite`) true false)
          (`SceneComponent.SetHiddenInGame` (`self.BootsSprite`) true false)
          (`SceneComponent.SetHiddenInGame` (`self.RobeSprite`) true false))
        (:`then_1`
          (goto _label))))
    (:`Hurt`
      (bind _bempty (`self.ModifyHealthBar` (* (- (`|GetArrayItem` _floats) (`self.Armor`)) -1.0)))
      (if _bempty
        (`/Game/AdvancedTurnBasedTileToolkit/Core/BPML_ATBTT.EndAction`)
        (`/Game/AdvancedTurnBasedTileToolkit/Core/BPML_ATBTT.SimpleQueue` "NewEnumerator1" self "Death")
        (else
          (`self.AnimateUnit` Action))))))

(event `self.MoveToIndex`
  (params (IndexPathEnd :type Integer) (PathsMap :type "Map of Integer to /Game/AdvancedTurnBasedTileToolkit/Core/Grid/FPathfindingNew Structure (by ref)"))
  (bind _pathindexes (`/Game/AdvancedTurnBasedTileToolkit/Core/Grid/BP_GridManager.FindPathToIndex` (`self.GridManagerRef`) PathsMap IndexPathEnd))
  (add `/Game/AdvancedTurnBasedTileToolkit/Core/Grid/BP_GridManager.OnUnitEnterTileSimulate` (`self.GridManagerRef`) (delegate `self.CustomEnterTileSimulate`))
  (`self.SimulateMove` _pathindexes)
  (remove `/Game/AdvancedTurnBasedTileToolkit/Core/Grid/BP_GridManager.OnUnitEnterTileSimulate` (`self.GridManagerRef`) (delegate `self.CustomEnterTileSimulate`)))

(event `self.CustomEnterTileSimulate`
  (params (Unit :type "/Game/AdvancedTurnBasedTileToolkit/Core/Units/BP_Unit Object Reference") (GridIndex :type Integer) (PathIndex :type Integer))
  (`/Game/AdvancedTurnBasedTileToolkit/Core/BPML_ATBTT.QueueAction` :`Executing Object` self :`Action Name` "MoveStep" :`Integers` (`|MakeArray` PathIndex) :`Vectors` (`|MakeArray` (`BlueprintMapLibrary.Map_Find` (`/Game/AdvancedTurnBasedTileToolkit/Core/Grid/BP_GridManager.GridLocations` (`self.GridManagerRef`)) GridIndex)))
  (`/Game/AdvancedTurnBasedTileToolkit/Core/Grid/BP_GridManager.InteractWithObjects` (`self.GridManagerRef`) GridIndex self null true "NewEnumerator1" PathIndex)
  (`/Game/AdvancedTurnBasedTileToolkit/Maps/2D/Core/BP_GridManager_2D.RevealTiles` (`self.GridManager2DRef`) GridIndex))

(event `Equip`
  (params (Damage :type "Float (double-precision)") (Armor :type "Float (double-precision)") (Sprite :type "PaperSprite Object Reference") (Type :type Integer) (Range :type Integer) (AttackSound :type "SoundBase Object Reference") (HitSound :type "SoundBase Object Reference") (Projectile :type "PaperSprite Object Reference"))
  (if (> Damage 0.0)
    (set `self.Damage` Damage))
  (set `self.Armor` (+ Armor (`self.Armor`)))
  (set `self.Range` Range)
  (`/Engine/EditorBlueprintResources/StandardMacros.IsValid` AttackSound
    (:`Is Valid`
      (set `self.AttackSound` AttackSound))
    (:`Is Not Valid`
      _))
  (`/Engine/EditorBlueprintResources/StandardMacros.IsValid` HitSound
    (:`Is Valid`
      (set `self.HitSound` HitSound))
    (:`Is Not Valid`
      _))
  (`/Engine/EditorBlueprintResources/StandardMacros.IsValid` Projectile
    (:`Is Valid`
      (set `self.Projectile` Projectile))
    (:`Is Not Valid`
      _))
  (`/Game/AdvancedTurnBasedTileToolkit/Core/BPML_ATBTT.QueueAction` :`Executing Object` self :`Action Name` "Equip" :`Instant Deactivate` true :`Integers` (`|MakeArray` Type) :`Objects` (`|MakeArray` Sprite :!type "Object Object Reference")))

(event `self.TakeDamage`
  (params (Damage :type "Float (single-precision)") (bAutoAnimate :type Boolean))
  (`parent.TakeDamage` (`KismetMathLibrary.FMax` (- Damage (`self.Armor`))) bAutoAnimate))

(fn `UserConstructionScript`
  (`parent.UserConstructionScript`))