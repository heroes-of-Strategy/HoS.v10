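; Mind control status effect for the turn-based tile toolkit that temporarily makes the affected unit an AI-controlled ally of the active unit.
; On activation it saves the unit's allied factions and AI flag, then copies the active unit's factions from the turn manager.
; Activation and turn start queue an action, with AnimateAction handling Mind Control particles and sound.
; Turn end restores the saved values and disables the effect.
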(event `self.RunOnTurnStart`
  (`/Game/AdvancedTurnBasedTileToolkit/Core/BPML_ATBTT.QueueAction` :`Executing Object` self :`Action Name` "MindControl" :`Units` (`|MakeArray` (`self.OwningUnit`)) :!label _label))

(event `self.Activate`
  (params (`Target Unit` :type "/Game/AdvancedTurnBasedTileToolkit/Core/Units/BP_Unit Object Reference"))
  (bind _owningunit (`self.OwningUnit`))
  (`parent.Activate` `Target Unit`)
  (set `self.OldAlliedFactions` (`/Game/AdvancedTurnBasedTileToolkit/Core/Units/BP_Unit.AlliedFactions` _owningunit))
  (set `self.bOldAIControlled` (`/Game/AdvancedTurnBasedTileToolkit/Core/Units/BP_Unit.bAIControlled` _owningunit))
  (bind _turnmanager (message `/Game/AdvancedTurnBasedTileToolkit/Core/BPI_Singletons.FindTurnManagerInState` (`GameplayStatics.GetGameState`)))
  (set `/Game/AdvancedTurnBasedTileToolkit/Core/Units/BP_Unit.AlliedFactions` (`/Game/AdvancedTurnBasedTileToolkit/Core/Units/BP_Unit.AlliedFactions` (`/Game/AdvancedTurnBasedTileToolkit/Core/BP_TurnManager.ActiveUnit` _turnmanager)) (`self.OwningUnit`))
  (set `/Game/AdvancedTurnBasedTileToolkit/Core/Units/BP_Unit.bAIControlled` true (`self.OwningUnit`))
  (goto _label))

(event `/Game/AdvancedTurnBasedTileToolkit/Core/BPI_Action.AnimateAction`
  (params (Action :type "/Game/AdvancedTurnBasedTileToolkit/Core/FAction Structure"))
  (bind (_executingobject _actionname _binstantdeactivate _atcustomindex _bwithprevious _activationdelay _booleans _integers _floats _strings _vectors _transforms _actors _units) (break `/Game/AdvancedTurnBasedTileToolkit/Core/FAction` Action))
  (bind _returnvalue (`self.K2_GetActorLocation` (`|GetArrayItem` _units)))
  (switch `name` _actionname
    (:`Default`
      (`parent.AnimateAction` Action))
    (:`MindControl`
      (`GameplayStatics.SpawnEmitterAtLocation` "/Game/AdvancedTurnBasedTileToolkit/Maps/Advanced/Abilities/PS_Posseser_Attach.PS_Posseser_Attach" _returnvalue)
      (`GameplayStatics.PlaySoundAtLocation` "/Game/AdvancedTurnBasedTileToolkit/Maps/Advanced/Abilities/A_MindControl.A_MindControl" _returnvalue (struct) 1.0 1.0 0.0 null null null)
      (`KismetSystemLibrary.Delay` 1.0)
      (`/Game/AdvancedTurnBasedTileToolkit/Core/BPML_ATBTT.EndAction`))))

(event `self.RunOnTurnEnd`
  (set `/Game/AdvancedTurnBasedTileToolkit/Core/Units/BP_Unit.AlliedFactions` (`self.OldAlliedFactions`) (`self.OwningUnit`))
  (set `/Game/AdvancedTurnBasedTileToolkit/Core/Units/BP_Unit.bAIControlled` (`self.bOldAIControlled`) (`self.OwningUnit`))
  (`self.Disable`))

(fn `UserConstructionScript`
  (`parent.UserConstructionScript`))